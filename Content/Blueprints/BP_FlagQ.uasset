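; BP_FlagQ is a quantum level-goal flag that spawns its own circuit manager and prepares a qubit in superposition, with extra setup in Level3.
; Tick shows N0 and S according to state probabilities, swapping materials while both are possible.
; Basis selects the measurement basis; Measure collapses the state and, if horizontal, moves the markers to E/W.
; Measurement also enables two trigger boxes that open the next level on player overlap.
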(event OnComponentBeginOverlap(Box)
  (params (OverlappedComponent :type Primitive%20Component%20Object%20Reference) (OtherActor :type Actor%20Object%20Reference) (OtherComp :type Primitive%20Component%20Object%20Reference) (OtherBodyIndex :type Integer) (bFromSweep :type Boolean) (SweepResult :type Hit%20Result%20Structure%20%28by%20ref%29))
  (Utilities|Casting|CastToBP_PlayerCharacter OtherActor)
  (Game|OpenLevel(byName) (Variables|Default|GetNext%20Level)))

(event OnComponentBeginOverlap(Box2)
  (params (OverlappedComponent :type Primitive%20Component%20Object%20Reference) (OtherActor :type Actor%20Object%20Reference) (OtherComp :type Primitive%20Component%20Object%20Reference) (OtherBodyIndex :type Integer) (bFromSweep :type Boolean) (SweepResult :type Hit%20Result%20Structure%20%28by%20ref%29))
  (Utilities|Casting|CastToBP_PlayerCharacter OtherActor)
  (Game|OpenLevel(byName) (Variables|Default|GetNext%20Level)))

(event Custom|Measure
  (bind _circuitmanager (Variables|Default|GetCircuitManager))
  (if (Variables|Default|GetCanMeasure)
    (if (Variables|Default|GetIsBasisIdentity)
      _
      (else
        (Default|ApplyGate _circuitmanager (Variables|Default|GetMeasureBasis) true false)))
    (bind _output_get (Default|Measure _circuitmanager))
    (Variables|Default|SetIsSuperPosition false)
    (if (== (.X (Math|Vector4|BreakVector4 _output_get)) 0.0)
      (Audio|PlaySound2D "/Game/JamStuff/Music/State1.State1" 1.0 1.0 0.0 0 0)
      (elif (== (.Y (Math|Vector4|BreakVector4 _output_get)) 0.0)
        (Audio|PlaySound2D "/Game/JamStuff/Music/State2.State2" 1.0 1.0 0.0 0 0)))))

(event Custom|EventFlagQuantum
  (params (IsHorizontal :type Boolean)))

(event Custom|Event%20Basis
  (params (Horizontally :type Boolean))
  (Variables|Default|SetIs%20Horizontal Horizontally)
  (if Horizontally
    (Variables|Default|SetMeasureBasis "NewEnumerator3")
    (Variables|Default|SetIsBasisIdentity false)
    (else
      (Variables|Default|SetIsBasisIdentity true)))
  (Variables|Default|SetCanMeasure true))

(event EventBeginPlay
  (bind _returnvalue (Game|SpawnActorfromClass "/Game/Blueprints/BP_CircuitManager.BP_CircuitManager_C" (Math|Transform|MakeTransform "0, 0, 0") "Undefined" 0 0))
  (bind _output_get (Variables|Default|SetCircuitManager _returnvalue))
  (bind _returnvalue_2 (Game|GetCurrentLevelName true))
  (if (Utilities|Enum|Equal(Enum) _returnvalue_2 "Level3")
    (Default|ApplyGate _output_get "NewEnumerator0" true false))
  (Default|ApplyGate _output_get "NewEnumerator3" true false)
  (Variables|Default|SetIsSuperPosition true))

(event EventTick
  (params (DeltaSeconds :type Float%20%28single-precision%29))
  (bind _box (Variables|Default|GetBox))
  (bind _output_get (Default|GetProbabilityVector (Variables|Default|GetCircuitManager)))
  (Transformation|SetRelativeScale3D (Variables|Default|GetN_0) (select (> (.x _output_get) 0.0) "5.000000,5.000000,5.000000" "0, 0, 0"))
  (Transformation|SetRelativeScale3D (Variables|Default|GetS) (select (> (.y _output_get) 0.0) "5.000000,5.000000,5.000000" "0, 0, 0"))
  (if (and (and (> (.x _output_get) 0.0) (> (.y _output_get) 0.0)) (and (< (.x _output_get) 1.0) (< (.y _output_get) 1.0)))
    (Rendering|Material|SetMaterial (Variables|Default|GetN_0) 0 "/Game/StarterContent/Materials/M_Water_Ocean.M_Water_Ocean")
    (else
      (Rendering|Material|SetMaterial (Variables|Default|GetS) 0 "/Game/JamStuff/Material/mat_cat.mat_cat")))
  (Transformation|SetRelativeScale3D _box (select (Variables|Default|GetIsSuperPosition) "0, 0, 0" "0.500000,0.500000,1.000000"))
  (Transformation|SetWorldLocation _box (Transformation|GetWorldLocation (Variables|Default|GetN_0)) false false)
  (Transformation|SetWorldLocation (Variables|Default|GetBox2) (Transformation|GetWorldLocation (Variables|Default|GetS)) false false)
  (if (not (Variables|Default|GetIsSuperPosition))
    (if (Variables|Default|GetIs%20Horizontal)
      (Transformation|SetWorldLocation (Variables|Default|GetN_0) (Transformation|GetWorldLocation (Variables|Default|GetE)) false false)
      (Transformation|SetWorldLocation (Variables|Default|GetS) (Transformation|GetWorldLocation (Variables|Default|GetW)) false false))))

(fn ConstructionScript)