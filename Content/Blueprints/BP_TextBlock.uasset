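; Word block for a rule-sentence puzzle, where lined-up blocks form commands that steer flag actors.
; The construction script labels the block and derives its grammar type from its word.
; On a check event, blocks lacking a left or upper neighbour gather a sentence through recursive line traces, though both paths scan horizontally.
; Two- and three-word parsers set quantum flag measurement basis, classical directions or superpositions; five-word parsing is empty.
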(event Custom|EventCheckSentence
  ;[1 1 1] Check if not Textblock on the left or above
  (bind _returnvalue (CallFunction|FindNeighbour true -1))
  (if _returnvalue
    _
    (else
      (bind _sentence (CallFunction|CheckSentence true))
      (CallFunction|ParseSentence _sentence)))
  (bind _returnvalue_2 (CallFunction|FindNeighbour false -1))
  (if (not _returnvalue_2)
    (bind _sentence_2 (CallFunction|CheckSentence true))
    (CallFunction|ParseSentence _sentence_2)))

(event EventBeginPlay
  (|CallParentFunction) ; This node is disabled and will not be called.\nDrag off pins to build functionality.
)

(event Collision|EventActorBeginOverlap
  (params (OtherActor :type Actor%20Object%20Reference)))

(event EventTick
  (params (DeltaSeconds :type Float%20%28single-precision%29))
  (|CallParentFunction DeltaSeconds))

(event Collision|EventActorEndOverlap
  (params (OtherActor :type Actor%20Object%20Reference)))

(fn ConstructionScript
  (bind _word (Variables|Default|GetWord))
  (|CallParentFunction)
  (Rendering|Components|TextRender|SetText (Variables|Default|GetTextRender) (Utilities|Text|ToText(String) (Utilities|String|EnumtoString _word)))
  (Variables|Default|SetWord_Type (Utilities|Select :Index _word :NewEnumerator10 "NewEnumerator11" :NewEnumerator11 "NewEnumerator10" :NewEnumerator12 "NewEnumerator12" :NewEnumerator13 "NewEnumerator12" :NewEnumerator14 "NewEnumerator12" :NewEnumerator15 "NewEnumerator12" :NewEnumerator16 "NewEnumerator17" :NewEnumerator17 "NewEnumerator18" :NewEnumerator18 "NewEnumerator18" :NewEnumerator19 "NewEnumerator12" :NewEnumerator20 "NewEnumerator12")))

(fn CheckSentence
  (params (Horizontal :type Boolean))
  (bind (_outhit _returnvalue) (CallFunction|FindNeighbour Horizontal 1))
  (if _returnvalue
    (bind _asbp_text_block (Utilities|Casting|CastToBP_TextBlock (.HitActor (Collision|BreakHitResult _outhit))))
    (bind _sentence (CallFunction|CheckSentence _asbp_text_block Horizontal))
    (Utilities|Array|Insert _sentence self)
    (return _sentence)
    (else
      (return (Utilities|Array|MakeArray self)))))

(fn ParseSentence
  (params (Sentence :type Array%20of%20BP%20Text%20Block%20Object%20References))
  ;[1 1 1] Check length
  (if (> (Utilities|Array|Length Sentence) 1)
    ;[1 1 1] Debug print
    (Variables|Default|SetDEBUG (Utilities|String|Append (Utilities|String|EnumtoString (Variables|Default|GetWord)) " : "))
    (for _array_element Sentence
      (Variables|Default|SetDEBUG (Utilities|String|Append (Variables|Default|GetDEBUG) (Utilities|String|EnumtoString (Variables|BP_TextBlock_C|GetWord _array_element)))))
    (Development|PrintString (Variables|Default|GetDEBUG))
    (switch int (Utilities|Array|Length Sentence)
      (:2
        (CallFunction|ParseSentenceLength2 Sentence Sentence))
      (:3
        (CallFunction|ParseSentenceLength3 Sentence))
      (:5
        (CallFunction|ParseSentenceLength5 Sentence)))))

(fn FindNeighbour
  (params (horizontal :type Boolean) (direction :type Integer))
  (bind _returnvalue (Transformation|GetActorLocation))
  (bind _returnvalue_2 (Transformation|GetActorLocation))
  (if horizontal
    ;[1 1 1] Check Horizontally
    (bind (_outhit _returnvalue_3) (Collision|LineTraceForObjects _returnvalue (+ _returnvalue (Math|Vector|MakeVector 0.0 (* direction (Variables|Default|GetRayLength)) 0.0)) (Utilities|Array|MakeArray "ObjectTypeQuery2") false 0 "ForDuration" true "(R=0.255208,G=0.000000,B=0.046962,A=1.000000)"))
    (return _outhit _returnvalue_3)
    (else
      ;[1 1 1] Check Vertically
      (bind (_outhit_2 _returnvalue_4) (Collision|LineTraceForObjects _returnvalue_2 (+ _returnvalue_2 (Math|Vector|MakeVector (* (* direction -1) (Variables|Default|GetRayLength)) 0.0 0.0)) (Utilities|Array|MakeArray "ObjectTypeQuery2") false 0 "ForDuration" true "(R=0.001730,G=0.000000,B=0.171875,A=1.000000)"))
      (return _outhit_2 _returnvalue_4))))

(fn ParseSentenceLength3
  (params (Sentence :type Array%20of%20BP%20Text%20Block%20Object%20References))
  (if (Math|Boolean|ANDBoolean (Utilities|Enum|Equal(Enum) (Variables|BP_TextBlock_C|GetWord_Type (Utilities|Array|Get(acopy) Sentence)) "NewEnumerator10") (Utilities|Enum|Equal(Enum) (Variables|BP_TextBlock_C|GetWord_Type (Utilities|Array|Get(acopy) Sentence 1)) "NewEnumerator11") (Utilities|Enum|Equal(Enum) (Variables|BP_TextBlock_C|GetWord_Type (Utilities|Array|Get(acopy) Sentence 2)) "NewEnumerator12"))
    ;[1 1 1] Grab the subject instances
    (switch Utilities|FlowControl|Switch|SwitchonWordList (Variables|BP_TextBlock_C|GetWord (Utilities|Array|Get(acopy) Sentence))
      (:NewEnumerator11
        (bind _outactors (Actor|GetAllActorsOfClass "/Game/Blueprints/BP_Flag.BP_Flag_C"))
        (LocalVariables|SetSubjectActors _outactors)
        (for _array_element (LocalVariables|GetSubjectActors)
          (switch Utilities|FlowControl|Switch|SwitchonWordList (Variables|BP_TextBlock_C|GetWord (Utilities|Array|Get(acopy) Sentence 2))
            (:NewEnumerator12
              ;[1 1 1] Handle Classical Flag
              (LocalVariables|SetCardinalDirection "North")
              (Default|EventFlagClassical _array_element (LocalVariables|GetCardinalDirection) :!label _label))
            (:NewEnumerator13
              (LocalVariables|SetCardinalDirection "South")
              (goto _label))
            (:NewEnumerator14
              (LocalVariables|SetCardinalDirection "East")
              (goto _label))
            (:NewEnumerator15
              (LocalVariables|SetCardinalDirection "West")
              (goto _label))
            (:NewEnumerator19
              ;[1 1 1] Handle Quantum Flag
              (LocalVariables|SetSuperpositionDirection true)
              (bind _outactors_2 (Actor|GetAllActorsOfClass "/Game/Blueprints/BP_FlagQ.BP_FlagQ_C" :!label _label_2))
              (for _array_element_2 _outactors_2
                (Default|EventFlagQuantum _array_element_2 (LocalVariables|GetSuperpositionDirection))))
            (:NewEnumerator20
              (LocalVariables|SetSuperpositionDirection false)
              (goto _label_2))))))))

(fn ParseSentenceLength5
  (params (Sentence :type Array%20of%20BP%20Text%20Block%20Object%20References)))

(fn SetEqual
  (params (set1 :type Set%20of%20Strings) (set2 :type Set%20of%20Strings))
  (bind _result (Utilities|Set|Difference set1 set2))
  (return (== (Utilities|Set|Length _result) 0)))

(fn ParseSentenceLength2
  (params (sentence :type Array%20of%20BP%20Text%20Block%20Object%20References))
  (if (and (Utilities|Enum|Equal(Enum) (Variables|BP_TextBlock_C|GetWord_Type (Utilities|Array|Get(acopy) sentence)) "NewEnumerator17") (Utilities|Enum|Equal(Enum) (Variables|BP_TextBlock_C|GetWord_Type (Utilities|Array|Get(acopy) sentence 1)) "NewEnumerator18"))
    ;[1 1 1] Grab the subject instances
    (switch Utilities|FlowControl|Switch|SwitchonWordList (Variables|BP_TextBlock_C|GetWord (Utilities|Array|Get(acopy) sentence))
      (:NewEnumerator16
        (bind _outactors (Actor|GetAllActorsOfClass "/Game/Blueprints/BP_Flag.BP_Flag_C"))
        (LocalVariables|SetSubjectActors _outactors)
        (for _array_element (LocalVariables|GetSubjectActors)
          (switch Utilities|FlowControl|Switch|SwitchonWordList (Variables|BP_TextBlock_C|GetWord (Utilities|Array|Get(acopy) sentence 1))
            (:NewEnumerator17
              ;[1 1 1] Handle Measurement
              (LocalVariables|SetMeasureDirection false))
            (:NewEnumerator18
              (LocalVariables|SetMeasureDirection true)))
          (bind _outactors_2 (Actor|GetAllActorsOfClass "/Game/Blueprints/BP_FlagQ.BP_FlagQ_C"))
          (for _array_element_2 _outactors_2
            (Default|EventBasis _array_element_2 (LocalVariables|GetMeasureDirection))))))))