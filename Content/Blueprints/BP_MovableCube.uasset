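; A pushable cube that slides when the player character overlaps its box and then has every BP_TextBlock check its sentence.
; PushCube snaps the player's forward vector to one of the cube's four horizontal axes and sets a target MoveUnits away.
; Tick interpolates toward that target at PushSpeed, while a short box trace along the player's forward cancels movement on hitting anything but the player.
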(event EventTick
  (params (DeltaSeconds :type Float%20%28single-precision%29))
  (AI|Navigation|StopMovement)
  (Transformation|SetActorLocation (Math|Interpolation|VInterpTo (Transformation|GetActorLocation) (Variables|Default|GetMoveLocation) DeltaSeconds (Variables|Default|GetPushSpeed)) false false))

(event EventBeginPlay
  (Variables|Default|SetMoveLocation (Transformation|GetActorLocation)))

(event OnComponentBeginOverlap(Box)
  (params (OverlappedComponent :type Primitive%20Component%20Object%20Reference) (OtherActor :type Actor%20Object%20Reference) (OtherComp :type Primitive%20Component%20Object%20Reference) (OtherBodyIndex :type Integer) (bFromSweep :type Boolean) (SweepResult :type Hit%20Result%20Structure%20%28by%20ref%29))
  (bind _asbp_player_character (Utilities|Casting|CastToBP_PlayerCharacter OtherActor))
  (CallFunction|PushCube (Transformation|GetActorForwardVector _asbp_player_character))
  (bind _outactors (Actor|GetAllActorsOfClass "/Game/Blueprints/BP_TextBlock.BP_TextBlock_C"))
  (for _array_element _outactors
    (Default|EventCheckSentence _array_element)))

(fn ConstructionScript)

(fn PushCube
  (params (ForwardVctor :type Vector))
  (bind _returnvalue (Transformation|GetActorRightVector))
  (bind _returnvalue_2 (Transformation|GetActorForwardVector))
  (bind _returnvalue_3 (* _returnvalue -1.0))
  (bind _returnvalue_4 (* _returnvalue_2 -1.0))
  (bind _returnvalue_5 (Math|Vector|DotProduct ForwardVctor _returnvalue_2))
  (bind _returnvalue_6 (Math|Vector|DotProduct ForwardVctor _returnvalue_3))
  (bind _returnvalue_7 (Math|Vector|DotProduct ForwardVctor _returnvalue_4))
  (bind _returnvalue_8 (Class|KismetMathLibrary|DegAcos _returnvalue_5))
  (bind _returnvalue_9 (Class|KismetMathLibrary|DegAcos _returnvalue_6))
  (bind _returnvalue_10 (Class|KismetMathLibrary|DegAcos _returnvalue_7))
  (bind _returnvalue_11 (Math|Float|Min(Float) _returnvalue_8 _returnvalue_10))
  (bind _returnvalue_12 (== _returnvalue_11 _returnvalue_10))
  (bind _returnvalue_13 (select _returnvalue_12 _returnvalue_4 _returnvalue_2))
  (bind _output_get (Variables|Default|SetMoveLocation (+ (Transformation|GetActorLocation) (* (select (< (Class|KismetMathLibrary|DegAcos (Math|Vector|DotProduct ForwardVctor _returnvalue_13)) 6e+01) _returnvalue_13 (select (== (Math|Float|Min(Float) (Class|KismetMathLibrary|DegAcos (Math|Vector|DotProduct ForwardVctor _returnvalue)) _returnvalue_9) _returnvalue_9) _returnvalue_3 _returnvalue)) (Variables|Default|GetMoveUnits)))))
  (return))