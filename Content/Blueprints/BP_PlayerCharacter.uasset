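; Player character that moves on the control-yaw plane, restarts the current level with R and triggers Measure on every BP_FlagQ with F.
; MoveForward and MoveRight axes feed AddMovementInput along flattened vectors from GetControlVectors.
; An alternative Movement graph gates SimpleMoveToLocation per direction through input actions, but its main entry is never run.
; R also plays a redo sound after requesting the level load.
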(event EventTick
  (params (DeltaSeconds :type Float%20%28single-precision%29)))

(event Input|AxisEvents|InputAxisMoveForward
  (params (AxisValue :type Float%20%28single-precision%29))
  (Pawn|Input|AddMovementInput (.Forward%20Vector (CallFunction|GetControlVectors false)) AxisValue false))

(event Input|AxisEvents|InputAxisMoveRight
  (params (AxisValue :type Float%20%28single-precision%29))
  (Pawn|Input|AddMovementInput (.Right%20Vector (CallFunction|GetControlVectors false)) AxisValue false))

(event Input|KeyboardEvents|F
  (params (Key :type Key%20Structure))
  (:Pressed
    (bind _outactors (Actor|GetAllActorsOfClass "/Game/Blueprints/BP_FlagQ.BP_FlagQ_C"))
    (for _array_element _outactors
      (Default|Measure _array_element))))

(event Input|KeyboardEvents|R
  (params (Key :type Key%20Structure))
  (:Pressed
    (bind _returnvalue (Game|GetCurrentLevelName true))
    (Game|OpenLevel(byName) (Utilities|String|StringToName _returnvalue))
    (Audio|PlaySound2D "/Game/JamStuff/Music/Redo_Level.Redo_Level" 1.0 1.0 0.0 0 0)))

(fn ConstructionScript)

(fn GetControlVectors
  (params (Reverse :type Boolean))
  (bind _returnvalue (Pawn|GetControlRotation :!class /Script/Engine.Pawn))
  (bind _yaw (Math|Rotator|BreakRotator _returnvalue))
  (bind _returnvalue_2 (Math|Rotator|MakeRotator 0.0 0.0 _yaw))
  (bind _returnvalue_3 (Math|Vector|GetForwardVector _returnvalue_2))
  (bind _returnvalue_4 (Math|Vector|GetRightVector _returnvalue_2))
  (return (select Reverse (* _returnvalue_3 -1.0) _returnvalue_3) (select Reverse (* _returnvalue_4 -1.0) _returnvalue_4)))

(event Input|ActionEvents|InputActionMoveForward
  (params (Key :type Key%20Structure))
  (:Pressed
    (Utilities|MoveinDirection (.Forward%20Vector (CallFunction|GetControlVectors false))) ; enters at Open
  )
  (:Released
    (Utilities|MoveinDirection (.Forward%20Vector (CallFunction|GetControlVectors false))) ; enters at Close
  ))

(event Input|ActionEvents|InputActionMoveBackward
  (params (Key :type Key%20Structure))
  (:Pressed
    (Utilities|MoveinDirection (.Forward%20Vector (CallFunction|GetControlVectors true))) ; enters at Open
  )
  (:Released
    (Utilities|MoveinDirection (.Forward%20Vector (CallFunction|GetControlVectors true))) ; enters at Close
  ))

(event Input|ActionEvents|InputActionMoveLeft
  (params (Key :type Key%20Structure))
  (:Pressed
    (Utilities|MoveinDirection (.Right%20Vector (CallFunction|GetControlVectors true))) ; enters at Open
  )
  (:Released
    (Utilities|MoveinDirection (.Right%20Vector (CallFunction|GetControlVectors true))) ; enters at Close
  ))

(event Input|ActionEvents|InputActionMoveRight
  (params (Key :type Key%20Structure))
  (:Pressed
    (Utilities|MoveinDirection (.Right%20Vector (CallFunction|GetControlVectors false))) ; enters at Open
  )
  (:Released
    (Utilities|MoveinDirection (.Right%20Vector (CallFunction|GetControlVectors false))) ; enters at Close
  ))