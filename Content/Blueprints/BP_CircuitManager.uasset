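; BP_CircuitManager is the Blueprint front end for a two-qubit circuit simulated in an attached Python component.
; ApplyGate builds a Python method name from the gate enum plus a 0/1 qubit suffix, using SelectedQubit unless Forced.
; Measure calls the Python collapse method; both operations then read get_probv into the four-component ProbVector and return it.
; A debug print of the probabilities exists but is not wired to any event.
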(event EventBeginPlay)

(event EventTick
  (params (DeltaSeconds :type Float%20%28single-precision%29)))

(fn ConstructionScript)

(fn AddQubitNumSuffix
  (params (Gate :type String) (QubitNum :type Boolean))
  (return (Utilities|String|Append Gate (select QubitNum "1" "0"))))

(fn GetProbabilityVector
  (bind _output_strings (Class|PythonComponent|CallPythonComponentMethodStringArray (Variables|Default|GetPython) "get_probv"))
  (bind _output_get (Variables|Default|SetProbVector (Math|Vector4|MakeVector4 (Math|Conversions|ToFloat(Integer) (Utilities|Array|Get(acopy) _output_strings)) (Math|Conversions|ToFloat(Integer) (Utilities|Array|Get(acopy) _output_strings 1)) (Math|Conversions|ToFloat(Integer) (Utilities|Array|Get(acopy) _output_strings 2)) (Math|Conversions|ToFloat(Integer) (Utilities|Array|Get(acopy) _output_strings 3)))))
  (return _output_get))

(fn DisplayProb
  (params (TextColor :type Linear%20Color%20Structure :default "(R=0.000000,G=1.000000,B=0.000000,A=1.000000)") (Duration :type Float%20%28single-precision%29))
  (bind _probvector (Variables|Default|GetProbVector))
  (bind (_x _y _z _w) (Math|Vector4|BreakVector4 _probvector))
  (Development|PrintString (Utilities|String|Append (Utilities|String|ToString(Vector2d) (Math|Vector2D|MakeVector2D _x _y)) " , " (Utilities|String|ToString(Vector2d) (Math|Vector2D|MakeVector2D _z _w))) true true TextColor Duration))

(fn ApplyGate
  (params (Gate :type Gate%20Enum :default "NewEnumerator0") (Forced? :type Boolean) (Qubit%20Num :type Boolean))
  (Class|PythonComponent|CallPythonComponentMethod (Variables|Default|GetPython) (PropertyFunctions|AddQubitNumSuffix (Utilities|String|EnumtoString Gate) (select Forced? Qubit%20Num (Variables|Default|GetSelectedQubit))))
  (bind _output_get (CircuitFunctions|GetProbabilityVector))
  (return _output_get))

(fn Measure
  (Class|PythonComponent|CallPythonComponentMethod (Variables|Default|GetPython) "collapse")
  (bind _output_get (CircuitFunctions|GetProbabilityVector))
  (return _output_get))